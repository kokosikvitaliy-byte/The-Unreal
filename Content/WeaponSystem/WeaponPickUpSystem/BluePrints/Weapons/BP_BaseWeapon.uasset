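; Base weapon Blueprint for the third-person character, leaving shoot and EndShoot empty.
; CreateShotTrace decrements magazine ammo and updates the character, then either auto-reloads at zero without firing or plays effects and multi-line traces from the follow camera.
; Each hit takes damage and spawns particles chosen by the actor's first tag.
; ReloadWeapon calls EndShoot, refills the magazine from reserve and triggers the character's Reload.
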(event Custom|CreateShotTrace
  (params (Range :type Float%20%28double-precision%29))
  (bind _shootarrow (Variables|Default|GetShootArrow))
  (bind _playercharacter (Variables|Default|GetPlayerCharacter))
  (bind _followcamera (Variables|/Game/ThirdPerson/Blueprints/BP_ThirdPersonCharacter.BP_ThirdPersonCharacter_C|GetFollowCamera _playercharacter))
  (bind _returnvalue (Transformation|GetWorldLocation _followcamera))
  (bind _output_get (Variables|Default|SetCurrentMagAmmo (Math|Integer|Clamp(Integer) (- (Variables|Default|GetCurrentMagAmmo) 1) 0 (Variables|Default|GetMaxMagAmmo))))
  (Default|UpdateAmmo (Variables|Default|GetPlayerCharacter) _output_get (Variables|Default|GetCurrentReserveAmmo))
  (if (<= _output_get 0)
    (CallFunction|ReloadWeapon)
    (else
      (Audio|PlaySound2D (Variables|Default|GetGunShotSoundEffect) 1.0 1.0 0.0 0 0)
      (Effects|SpawnEmitterAttached "/Game/Realistic_Starter_VFX_Pack_Vol2/Particles/Explosion/P_Explosion_Big_A.P_Explosion_Big_A" _shootarrow "None" "0, 0, 0" "0, 0, 0" "0.030000,0.030000,0.030000")
      (bind (_outhits _returnvalue_2) (Class|KismetSystemLibrary|LineTraceMultiforObjects _returnvalue (+ _returnvalue (* (Math|Vector|GetForwardVector (Transformation|GetWorldRotation _followcamera)) Range)) (Utilities|Array|MakeArray "ObjectTypeQuery3" "ObjectTypeQuery1") false 0 "None" true))
      (if _returnvalue_2
        (bind _array_element (Utilities|Array|ForEachLoopwithBreak _outhits)
          (:LoopBody
            (CallFunction|SpawnHitParticles (Utilities|Array|Get(acopy) (Variables|/Script/Engine.Actor|GetTags (.HitActor (Collision|BreakHitResult _array_element)))) (.Location (Collision|BreakHitResult _array_element)) (Transformation|GetWorldRotation _shootarrow))
            (Game|Damage|ApplyDamage (.HitActor (Collision|BreakHitResult _array_element)) (Variables|Default|GetDamage) 0 0)))))))

(event Custom|shoot)

(event Custom|EndShoot)

(event Custom|SpawnHitParticles
  (params (TagName :type Name) (Location :type Vector) (ArrowRotation :type Rotator))
  (bind (_roll _pitch _yaw) (Math|Rotator|BreakRotator ArrowRotation))
  (switch name TagName
    (:Default
      (Variables|Default|SetHitParticles "/Game/Realistic_Starter_VFX_Pack_Vol2/Particles/Destruction/P_Destruction_Concrete.P_Destruction_Concrete"))
    (:Brick
      (Variables|Default|SetHitParticles "/Game/Realistic_Starter_VFX_Pack_Vol2/Particles/Destruction/P_Destruction_Concrete.P_Destruction_Concrete"))
    (:Metal
      (Variables|Default|SetHitParticles "/Game/Realistic_Starter_VFX_Pack_Vol2/Particles/Destruction/P_Destruction_Metal.P_Destruction_Metal"))
    (:Wood
      (Variables|Default|SetHitParticles "/Game/Realistic_Starter_VFX_Pack_Vol2/Particles/Destruction/P_Destruction_Wood.P_Destruction_Wood"))
    (:Glass
      (Variables|Default|SetHitParticles "/Game/Realistic_Starter_VFX_Pack_Vol2/Particles/Destruction/P_Destruction_Glass.P_Destruction_Glass"))
    (:Enemy
      (Variables|Default|SetHitParticles "/Game/Realistic_Starter_VFX_Pack_Vol2/Particles/Blood/P_Blood_Splat_Cone.P_Blood_Splat_Cone")))
  (Effects|SpawnEmitteratLocation (Variables|Default|GetHitParticles) Location (Math|Rotator|MakeRotator _roll (+ _pitch 9e+01) _yaw) "0.200000,0.200000,0.200000"))

(event Custom|ReloadWeapon
  (if (not (== (Variables|Default|GetCurrentMagAmmo) (Variables|Default|GetMaxMagAmmo)))
    (if (not (<= (Variables|Default|GetCurrentReserveAmmo) 0))
      (CallFunction|EndShoot)
      (bind _output_get (Variables|Default|SetNeededAmmo (- (Variables|Default|GetMaxMagAmmo) (Variables|Default|GetCurrentMagAmmo))))
      (if (>= (Variables|Default|GetCurrentReserveAmmo) _output_get)
        (Variables|Default|SetCurrentMagAmmo (+ (Variables|Default|GetNeededAmmo) (Variables|Default|GetCurrentMagAmmo)))
        (Variables|Default|SetCurrentReserveAmmo (- (Variables|Default|GetCurrentReserveAmmo) (Variables|Default|GetNeededAmmo)))
        (Default|Reload (Variables|Default|GetPlayerCharacter))
        (else
          (Variables|Default|SetCurrentMagAmmo (+ (Variables|Default|GetCurrentReserveAmmo) (Variables|Default|GetCurrentMagAmmo)))
          (Variables|Default|SetCurrentReserveAmmo 0)
          (Default|Reload (Variables|Default|GetPlayerCharacter)))))))

(event EventBeginPlay
  (bind _asbp_third_person_character (Utilities|Casting|CastToBP_ThirdPersonCharacter (Game|GetPlayerCharacter 0)))
  (Variables|Default|SetPlayerCharacter _asbp_third_person_character))

(fn ConstructionScript)