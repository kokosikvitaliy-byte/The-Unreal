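; BP_enemyTest is a test enemy that chases the first player and plays an attack animation when it gets close.
; From BeginPlay, ChasePlayer runs AI MoveTo on the player character; success plays the attack montage on the mesh and restarts the chase after a short delay.
; A failed move retries immediately, with no delay.
; The attack only plays the montage, with no damage logic.
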(event Custom|ChasePlayer
  (AI|AIMoveTo self "0, 0, 0" (Game|GetPlayerCharacter 0) 1.5e+02 false
    (:OnSuccess
      (CallFunction|Attack)
      (Utilities|FlowControl|Delay 2.0)
      (CallFunction|ChasePlayer))
    (:OnFail
      (CallFunction|ChasePlayer))))

(event Custom|Attack
  (Animation|Montage|PlayMontage (Variables|Character|GetMesh) "/Game/Characters/Mannequins/Anims/Unarmed/Attack/MM_Attack_01_Montage.MM_Attack_01_Montage"))

(event EventBeginPlay
  (CallFunction|ChasePlayer))

(fn ConstructionScript)